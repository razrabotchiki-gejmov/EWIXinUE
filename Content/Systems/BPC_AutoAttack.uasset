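; Actor component that runs auto-attacks from its owner against a Target, driven by external Attack calls supplying stats and delta time.
; In range, a cooldown derived from attack speed and base attack time gates random damage sent via TakeDamageMessage; out of range, GoToTarget issues a move.
; Crits use pseudo-random distribution, with chance growing per non-crit attack, and an active Blindness response can make attacks miss.
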(event EventBeginPlay)

(event EventTick
  (params (DeltaSeconds :type Float%20%28single-precision%29)))

(fn AutoAttackCheck
  (params (Target :type Actor%20Object%20Reference) (AttackDealer :type Actor%20Object%20Reference) (AttackRange :type Float%20%28double-precision%29))
  (bind _output_get (Variables|Default|SetTarget Target))
  (bind _output_get_2 (Variables|Default|SetInRange (<= (Math|Vector|VectorLength (- (Transformation|GetActorLocation _output_get) (Transformation|GetActorLocation AttackDealer))) AttackRange)))
  (return _output_get_2))

(fn CheckforNewAttack
  (params (AttackSpeed :type Float%20%28double-precision%29) (BaseAttackTime :type Float%20%28double-precision%29) (AttackRange :type Float%20%28double-precision%29) (CritChance :type Float%20%28double-precision%29))
  (bind _inrange (CallFunction|AutoAttackCheck (Variables|Default|GetTarget) (Components|GetOwner) AttackRange))
  (if _inrange
    (bind _canattack (CallFunction|CanAttack AttackSpeed BaseAttackTime))
    (if _canattack
      (Variables|Default|SetAttackCooldown 0.0)
      (bind _hascrit (CallFunction|CritCheck CritChance)))
    (return _inrange _canattack _hascrit)))

(fn Attack
  (params (DamageRange :type Array%20of%20Floats%20%28double-precision%29) (CritMultiplier :type Float%20%28double-precision%29) (AttackSpeed :type Float%20%28double-precision%29) (BaseAttackTime :type Float%20%28double-precision%29) (AttackRange :type Float%20%28double-precision%29) (CritChance :type Float%20%28double-precision%29) (Responce :type S%20Responce%20Structure) (DeltaSeconds :type Float%20%28double-precision%29))
  (bind (_responcetype _responcetime _active) (Utilities|Struct|BreakS_Responce Responce))
  (Utilities|IsValid (Variables|Default|GetTarget)
    (:Is%20Valid
      (bind (_inrange _canattack _hascrit) (CallFunction|CheckforNewAttack AttackSpeed BaseAttackTime AttackRange CritChance))
      (if _inrange
        (if _canattack
          (if (and (== _responcetype 7) _active)
            (if (> (Math|Random|RandomFloat) 0.3)
              (if _hascrit :!label _label
                (bind _damage (CallFunction|RandomDamage DamageRange))
                (Development|PrintString "Crit!")
                (Class|BPIDamagalbe|TakeDamage(Message) (Variables|Default|GetTarget) (Utilities|Struct|MakeS_DamageInfo (* _damage CritMultiplier) "NewEnumerator1" "NewEnumerator1" 0.0 false 0.0 true) (Components|GetOwner))
                (else
                  (bind _damage_2 (CallFunction|RandomDamage DamageRange))
                  (Class|BPIDamagalbe|TakeDamage(Message) (Variables|Default|GetTarget) (Utilities|Struct|MakeS_DamageInfo _damage_2 "NewEnumerator1" "NewEnumerator1" 0.0 false 0.0 true) (Components|GetOwner))))
              (else
                (Development|PrintString "Miss!")))
            (else
              (goto _label)))
          (else
            (CallFunction|TimeforAttack DeltaSeconds)))
        (else
          (CallFunction|GotoTarget))))))

(fn CanAttack
  (params (AttackSpeed :type Float%20%28double-precision%29) (BaseAttackTime :type Float%20%28double-precision%29))
  (return (>= (Variables|Default|GetAttackCooldown) (/ 1.0 (/ (/ AttackSpeed 1e+02) BaseAttackTime)))))

(fn TimeforAttack
  (params (DeltaSeconds :type Float%20%28double-precision%29))
  (Variables|Default|SetAttackCooldown (+ DeltaSeconds (Variables|Default|GetAttackCooldown))))

(fn CritCheck
  (params (CritChance :type Float%20%28double-precision%29))
  (if (< (Math|Random|RandomFloat) (* (Variables|Default|GetNoCrit) (/ CritChance 3.6e+02)))
    (Variables|Default|SetNoCrit 1)
    (return true)
    (else
      (Variables|Default|SetNoCrit (+ (Variables|Default|GetNoCrit) 1))
      (return false))))

(fn RandomDamage
  (params (DamageRange :type Array%20of%20Floats%20%28double-precision%29))
  (return (Math|Conversions|ToFloat(Integer) (Math|Float|Floor (Math|Random|RandomFloatinRange (Utilities|Array|Get(acopy) DamageRange) (Utilities|Array|Get(acopy) DamageRange 1))))))

(fn GotoTarget
  (bind _returnvalue (Components|GetOwner))
  (bind _asbp_top_down_controller (Utilities|Casting|CastToBP_TopDownController _returnvalue)
    (:then
      (Default|Moveto _asbp_top_down_controller "0, 0, 0"))
    (:CastFailed
      (AI|Navigation|SimpleMovetoActor (AI|GetAIController _returnvalue)))))
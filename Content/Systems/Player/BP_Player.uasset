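; Player character with timed passive gold, a stats widget, ragdoll death, auto-attacks and five skills.
; Damage, auto-attack, skill and characteristics components hold the logic, with wrapper functions exposing health, mana, healing and damage.
; Tick reads the damage response to apply knockback or disable movement, otherwise running auto-attacks with crit and miss rolls.
; Q/W/E/R/T open gates that left click fires: area, target, heal, projectile and cone skills.
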(event Custom|PassiveGold
  (bind _output_get (Variables|Default|SetGold (+ (Variables|Default|GetGold) 0.6)))
  (Development|PrintString (Utilities|String|Append "GOLD: " (Utilities|String|ToString(Integer) (Math|Float|Truncate _output_get)))))

(event Custom|AutoAttack
  (bind _bpc_damagesystem (Variables|Default|GetBPC_DamageSystem))
  (bind _bpc_autoattack (Variables|Default|GetBPC_AutoAttack))
  (bind _responce (Variables|/Game/Systems/BPC_DamageSystem.BPC_DamageSystem_C|GetResponce _bpc_damagesystem))
  (bind (_responcetype _responcetime _active) (Utilities|Struct|BreakS_Responce _responce))
  (Utilities|IsValid (Variables|/Game/Systems/BPC_AutoAttack.BPC_AutoAttack_C|GetTarget _bpc_autoattack)
    (:Is%20Valid
      (bind (_canattack _inrange _hascrit) (Default|CheckforNewAttack _bpc_autoattack (Variables|AutoAttack|GetAttackSpeed) (Variables|AutoAttack|GetBaseAttackTime) (Variables|AutoAttack|GetAttackRange) (Variables|Stats|GetCritChance)))
      (Variables|AutoAttack|SetTargetInRange _inrange)
      (if _canattack
        (if (and (== _responcetype 7) _active)
          (if (> (Math|Random|RandomFloat) 0.3)
            (if _hascrit :!label _label
              (bind _newparam (CallFunction|NewFunction))
              (Development|PrintString "Crit!")
              (Default|Attack _bpc_autoattack (Utilities|Struct|MakeS_DamageInfo (* _newparam (Variables|Stats|GetCritMultiplier)) "NewEnumerator1" "NewEnumerator1"))
              (else
                (bind _newparam_2 (CallFunction|NewFunction))
                (Default|Attack _bpc_autoattack (Utilities|Struct|MakeS_DamageInfo _newparam_2 "NewEnumerator1" "NewEnumerator1"))))
            (else
              (Development|PrintString "Miss!")))
          (else
            (goto _label)))))))

(event Custom|OnDeath
  (bind _mesh (Variables|Character|GetMesh))
  (Physics|SetSimulatePhysics _mesh true)
  (Collision|SetCollisionEnabled _mesh "QueryAndPhysics")
  (Input|DisableInput (Game|GetPlayerController 0)))

(event Custom|RecMana
  (CallFunction|RecoveryMana (/ (Variables|/Game/Systems/BPC_Characteristics.BPC_Characteristics_C|GetRegenMana (Variables|Default|GetBPC_Characteristics)) 1e+01)))

(event Custom|OnHit
  (params (DamageResponse :type E_DamageResponse%20Enum :default "NewEnumerator0"))
  (Development|PrintString (Utilities|String|EnumtoString DamageResponse)))

(event Custom|HealSkillAOE
  (params (Actor :type Actor%20Object%20Reference))
  (bind _newhealth (Class|BPIDamagalbe|Heal(Message) Actor 1e+01))
  (Variables|/Game/Systems/BPC_DamageSystem.BPC_DamageSystem_C|SetHealth (Variables|Default|GetBPC_DamageSystem) _newhealth))

(event EventBeginPlay
  (Utilities|Time|SetTimerbyEvent (EventDispatchers|CreateEvent :!event Custom|RecMana) 0.1 true)
  (Utilities|Time|SetTimerbyEvent (EventDispatchers|CreateEvent :!event Healing) 0.1 true)
  (Utilities|FlowControl|Sequence
    (:then_0
      (Utilities|Time|SetTimerbyEvent (delegate Custom|PassiveGold) 1.0 true))
    (:then_1
      (bind _returnvalue (UserInterface|CreateWidget "/Game/Systems/Interface123.Interface123_C" 0 self))
      (bind _output_get (Variables|Interface|SetInterfaceWidget _returnvalue))
      (UserInterface|Viewport|AddtoViewport _returnvalue 0))))

(event EventTick
  (params (DeltaSeconds :type Float%20%28single-precision%29))
  (bind _returnvalue (Game|GetPlayerController 0))
  (bind _charactermovement (Variables|Character|GetCharacterMovement))
  (bind _bpc_damagesystem (Variables|Default|GetBPC_DamageSystem))
  (bind _bpc_damagesystem_2 (Variables|Default|GetBPC_DamageSystem))
  (bind _attackerinfo (Variables|/Game/Systems/BPC_DamageSystem.BPC_DamageSystem_C|GetAttackerInfo _bpc_damagesystem))
  (if (== (.ResponceType (Utilities|Struct|BreakS_Responce (Variables|/Game/Systems/BPC_DamageSystem.BPC_DamageSystem_C|GetResponce _bpc_damagesystem_2))) 5)
    (Transformation|SetActorLocation (+ (Transformation|GetActorLocation) (* (Transformation|GetActorForwardVector (.Attacker (Utilities|Struct|BreakS_AttackerInfo (Utilities|Array|Get(acopy) _attackerinfo (Utilities|Array|LastIndex _attackerinfo))))) "30.000000,30.000000,30.000000")) true false)
    (Variables|/Game/Systems/BPC_DamageSystem.BPC_DamageSystem_C|SetResponce _bpc_damagesystem_2 ""))
  (if (== (.ResponceType (Utilities|Struct|BreakS_Responce (Variables|/Game/Systems/BPC_DamageSystem.BPC_DamageSystem_C|GetResponce _bpc_damagesystem_2))) 2)
    (if (.Active (Utilities|Struct|BreakS_Responce (Variables|/Game/Systems/BPC_DamageSystem.BPC_DamageSystem_C|GetResponce _bpc_damagesystem_2)))
      (Input|DisableInput _returnvalue)
      (Pawn|Components|CharacterMovement|DisableMovement _charactermovement :!label _label)
      (Variables|Default|SetPreviuosMovement (Variables|/Script/Engine.CharacterMovementComponent|GetMovementMode _charactermovement))
      (Variables|Default|SetDisabledMovement true)
      (Default|CountResponce (Variables|Default|GetBPC_DamageSystem) DeltaSeconds)
      (else
        (Input|EnableInput _returnvalue :!label _label_2)
        (if (Variables|Default|GetDisabledMovement)
          (Pawn|Components|CharacterMovement|SetMovementMode _charactermovement (Variables|Default|GetPreviuosMovement) 0))
        (Rendering|Debug|DrawDebugCircle (Transformation|GetActorLocation) 1e+02 12 "(R=1.000000,G=0.000000,B=0.198145,A=1.000000)" 0.0 2.0 "0.000000,1.000000,0.000000" "1.000000,0.000000,0.000000" true)
        (Default|TimeforAttack (Variables|Default|GetBPC_AutoAttack) DeltaSeconds)
        (if (Variables|AutoAttack|GetTargetInRange)
          (CallFunction|AutoAttack))))
    (elif (== (.ResponceType (Utilities|Struct|BreakS_Responce (Variables|/Game/Systems/BPC_DamageSystem.BPC_DamageSystem_C|GetResponce _bpc_damagesystem_2))) 4)
      (if (.Active (Utilities|Struct|BreakS_Responce (Variables|/Game/Systems/BPC_DamageSystem.BPC_DamageSystem_C|GetResponce _bpc_damagesystem_2)))
        (goto _label)
        (else
          (goto _label_2)))
      (else
        (Default|CountResponce (Variables|Default|GetBPC_DamageSystem) DeltaSeconds)
        (goto _label_2)))))

(event Input|KeyboardEvents|Q
  (params (Key :type Key%20Structure :default "None"))
  (bind _returnvalue (Game|GetPlayerController 0))
  (bind _array (Utilities|Array|MakeArray "ObjectTypeQuery1"))
  (bind _hitresult (Class|PlayerController|GetHitResultUnderCursorforObjects _returnvalue _array true))
  (bind _location (Collision|BreakHitResult _hitresult))
  (:Pressed
    (bind _cancast (Utilities|CanCastSpell (Variables|/Game/Systems/BPC_DamageSystem.BPC_DamageSystem_C|GetResponce (Variables|Default|GetBPC_DamageSystem)))
      (:Go
        (if _cancast
          (Utilities|FlowControl|Gate true) ; enters at Open
        )))))

(event Input|MouseEvents|LeftMouseButton
  (params (Key :type Key%20Structure :default "None"))
  (bind _returnvalue (Game|GetPlayerController 0))
  (bind _array (Utilities|Array|MakeArray "ObjectTypeQuery1"))
  (bind _hitresult (Class|PlayerController|GetHitResultUnderCursorforObjects _returnvalue _array true))
  (bind _location (Collision|BreakHitResult _hitresult))
  (:Pressed
    (Utilities|FlowControl|Gate true :!label _label
      (:Exit
        (Development|PrintString "Skill activated")
        (Development|PrintString (Utilities|String|ToString(Vector) _location))
        (Default|AoeDamage (Variables|Default|GetBPC_SkillSystem) (Utilities|Struct|MakeS_DamageInfo 15.0 "NewEnumerator2" "NewEnumerator1" 0.0 true 0.0 true) _location (Game|GetInstigator) 1e+02 0.2 true true))))
  (:Released
    (goto _label Close)))

(event Input|KeyboardEvents|W
  (params (Key :type Key%20Structure :default "None"))
  (:Pressed
    (bind _cancast (Utilities|CanCastSpell (Variables|/Game/Systems/BPC_DamageSystem.BPC_DamageSystem_C|GetResponce (Variables|Default|GetBPC_DamageSystem)))
      (:Go
        (if _cancast
          (Utilities|FlowControl|Gate true) ; enters at Open
        )))))

(event Input|MouseEvents|LeftMouseButton
  (params (Key :type Key%20Structure :default "None"))
  (:Pressed
    (Utilities|FlowControl|Gate true :!label _label
      (:Exit
        (Development|PrintString "Skill activated")
        (Default|TargetDamage (Variables|Default|GetBPC_SkillSystem) (Utilities|Struct|MakeS_DamageInfo 2e+01 "NewEnumerator2" "NewEnumerator1" 0.0 true)))))
  (:Released
    (goto _label Close)))

(event Input|KeyboardEvents|T
  (params (Key :type Key%20Structure :default "None"))
  (:Pressed
    (bind _cancast (Utilities|CanCastSpell (Variables|/Game/Systems/BPC_DamageSystem.BPC_DamageSystem_C|GetResponce (Variables|Default|GetBPC_DamageSystem)))
      (:Go
        (if _cancast
          (Utilities|FlowControl|Gate true) ; enters at Open
        )))))

(event Input|KeyboardEvents|R
  (params (Key :type Key%20Structure :default "None"))
  (:Pressed
    (bind _cancast (Utilities|CanCastSpell (Variables|/Game/Systems/BPC_DamageSystem.BPC_DamageSystem_C|GetResponce (Variables|Default|GetBPC_DamageSystem)))
      (:Go
        (if _cancast
          (Utilities|FlowControl|Gate true) ; enters at Open
        )))))

(event Input|MouseEvents|LeftMouseButton
  (params (Key :type Key%20Structure :default "None"))
  (:Pressed
    (Utilities|FlowControl|Gate true :!label _label
      (:Exit
        (Development|PrintString "Skill activated")
        (bind _projectiletoignore (Default|ProjectileDamage (Variables|Default|GetBPC_SkillSystem) (Utilities|Struct|MakeS_DamageInfo 3e+01 "NewEnumerator3" "NewEnumerator1") (Transformation|GetActorLocation) (Variables|Actor|GetInstigator) 2e+02 false))
        (Collision|IgnoreActorwhenMoving (Variables|Collision|GetCapsuleComponent) _projectiletoignore true))))
  (:Released
    (goto _label Close)))

(event Input|MouseEvents|LeftMouseButton
  (params (Key :type Key%20Structure :default "None"))
  (:Pressed
    (Utilities|FlowControl|Gate true :!label _label
      (:Exit
        (Development|PrintString "Skill activated")
        (Default|ConeDamage (Variables|Default|GetBPC_SkillSystem) (Utilities|Struct|MakeS_DamageInfo 2e+01 "NewEnumerator1" "NewEnumerator1" 0.0 true 0.0 true) (Transformation|GetActorLocation) (Variables|Actor|GetInstigator) 1e+01 1e+01 0.2 true))))
  (:Released
    (goto _label Close)))

(event Input|KeyboardEvents|E
  (params (Key :type Key%20Structure :default "None"))
  (bind _returnvalue (Game|GetInstigator))
  (bind _returnvalue_2 (Transformation|GetActorLocation))
  (:Pressed
    (Utilities|CanCastSpell (Variables|/Game/Systems/BPC_DamageSystem.BPC_DamageSystem_C|GetResponce (Variables|Default|GetBPC_DamageSystem))
      (:Go
        (if true
          (Utilities|FlowControl|Gate true) ; enters at Open
        )))))

(event Input|MouseEvents|LeftMouseButton
  (params (Key :type Key%20Structure :default "None"))
  (bind _returnvalue (Game|GetInstigator))
  (bind _returnvalue_2 (Transformation|GetActorLocation))
  (:Pressed
    (Utilities|FlowControl|Gate true :!label _label
      (:Exit
        (Development|PrintString "Skill activated")
        (Development|PrintString (Utilities|String|ToString(Vector) _returnvalue_2))
        (bind _returnvalue_3 (Game|SpawnActorfromClass "/Game/AOE/BP_AOE_Heal.BP_AOE_Heal_C" (Math|Transform|MakeTransform _returnvalue_2 "0, 0, 0" "1.000000,1.000000,1.000000") "Undefined" "MultiplyWithRoot" _returnvalue 1e+02 false true 0.2 _returnvalue))
        (EventDispatchers|AssignOnAoeOverlapActor _returnvalue_3 (delegate Custom|HealSkillAOE)))))
  (:Released
    (goto _label Close)))

(fn ConstructionScript
  (bind _bpc_damagesystem (Variables|Default|GetBPC_DamageSystem))
  (EventDispatchers|BindEventtoOnDeath _bpc_damagesystem (EventDispatchers|CreateEvent :!event Custom|OnDeath))
  (EventDispatchers|BindEventtoOnDamageResponse _bpc_damagesystem (EventDispatchers|CreateEvent :!event Custom|OnHit)))

(fn SkillCooldown
  (params (SkillCooldown :type Niagara%20Data%20Interface%20Array%20Float%20Object%20Reference) (Delta :type Float%20%28double-precision%29))
  (bind _floatdata (Variables|/Script/Niagara.NiagaraDataInterfaceArrayFloat|GetFloatData SkillCooldown))
  (for (_array_element _array_index) _floatdata
    (Utilities|Array|SetArrayElem _floatdata _array_index (+ _array_element Delta))))

(fn NewFunction
  (bind _damage (Variables|Stats|GetDamage))
  (return (Math|Conversions|ToFloat(Integer) (Math|Float|Floor (Math|Random|RandomFloatinRange (Utilities|Array|Get(acopy) _damage) (Utilities|Array|Get(acopy) _damage 1))))))

(fn Healing
  (bind _newhealth (CallFunction|Heal (/ (Variables|/Game/Systems/BPC_Characteristics.BPC_Characteristics_C|GetRegenHealth (Variables|Default|GetBPC_Characteristics)) 1e+01)))
  (Variables|/Game/Systems/BPC_DamageSystem.BPC_DamageSystem_C|SetHealth (Variables|Default|GetBPC_DamageSystem) _newhealth))

(fn RecoveryMana
  (params (Amount :type Float%20%28double-precision%29))
  (bind _bpc_characteristics (Variables|Default|GetBPC_Characteristics))
  (Variables|/Game/Systems/BPC_Characteristics.BPC_Characteristics_C|SetMana _bpc_characteristics (Math|Float|Clamp(Float) (+ Amount (Variables|/Game/Systems/BPC_Characteristics.BPC_Characteristics_C|GetMana _bpc_characteristics)) 0.0 (Variables|/Game/Systems/BPC_Characteristics.BPC_Characteristics_C|GetMaxMana _bpc_characteristics))))

(fn GetCurrentHealth
  (return (Variables|/Game/Systems/BPC_DamageSystem.BPC_DamageSystem_C|GetHealth (Variables|Default|GetBPC_DamageSystem))))

(fn GetCurrentMana
  (return (Variables|/Game/Systems/BPC_Characteristics.BPC_Characteristics_C|GetMana (Variables|Default|GetBPC_Characteristics))))

(fn GetMaxHealth
  (return (Variables|/Game/Systems/BPC_DamageSystem.BPC_DamageSystem_C|GetMaxHealth (Variables|Default|GetBPC_DamageSystem))))

(fn GetMaxMana
  (return (Variables|/Game/Systems/BPC_Characteristics.BPC_Characteristics_C|GetMaxMana (Variables|Default|GetBPC_Characteristics))))

(fn Heal
  (params (Amount :type Float%20%28double-precision%29))
  (bind _newhealth (Default|Heal (Variables|Default|GetBPC_DamageSystem) Amount))
  (return _newhealth))

(fn TakeDamage
  (params (DamageInfo :type S%20Damage%20Info%20Structure) (Attacker :type Actor%20Object%20Reference))
  (bind _wasdamaged (Default|TakeDamage (Variables|Default|GetBPC_DamageSystem) DamageInfo (Variables|/Game/Systems/BPC_Characteristics.BPC_Characteristics_C|GetArmor (Variables|Default|GetBPC_Characteristics)) (Variables|Stats|GetMagicResistance) (Variables|Effects|GetHasMagicInvulnerability) Attacker))
  (return _wasdamaged))
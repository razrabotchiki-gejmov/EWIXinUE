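; Character attribute component that derives health, mana, regeneration, attack, armor, magic resistance and attack speed.
; Power, Dexterity and Intelligence drive most derived stats via fixed formulas, with MainStat choosing the attack bonus; attack speed uses only its base values.
; RecheckCharacteristics recomputes everything on BeginPlay and LevelUp, then copies MaxHealth to the player pawn's damage system.
; BeginPlay then fills Health and Mana, while LevelUp adds per-level gains and a level point.
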(event EventBeginPlay
  (CallFunction|RecheckCharacteristics)
  (Variables|Health|SetHealth (Variables|Health|GetMaxHealth))
  (Variables|Mana|SetMana (Variables|Mana|GetMaxMana)))

(event EventTick
  (params (DeltaSeconds :type Float%20%28single-precision%29)))

(fn SetMaxHeath
  (Variables|Health|SetMaxHealth (+ (Variables|basic|GetBasicHealth) (* (Math|Float|Floor (Variables|Stats|GetPower)) 19.0))))

(fn SetRegenHeath
  (Variables|Health|SetRegenHealth (+ (Variables|Basic|GetBasicRegenHealth) (* (Variables|Stats|GetPower) 0.1))))

(fn SetMaxMana
  (Variables|Mana|SetMaxMana (* (Math|Float|Floor (Variables|Stats|GetIntelligence)) 13.0)))

(fn SetRegenMana
  (Variables|Mana|SetRegenMana (* (Variables|Stats|GetIntelligence) 0.04)))

(fn SetAttack
  (bind _basicattack (Variables|Basic|GetBasicAttack))
  (bind _attack (Variables|Attack|GetAttack))
  (bind _statsinarray (Variables|Basic|GetStatsInArray))
  (bind _mainstat (Variables|Basic|GetMainStat))
  (bind _output (Utilities|Array|Get(acopy) _statsinarray _mainstat))
  (Utilities|Array|SetArrayElem _attack 0 (+ (Utilities|Array|Get(acopy) _basicattack) _output))
  (Utilities|Array|SetArrayElem _attack 1 (+ _output (Utilities|Array|Get(acopy) _basicattack 1))))

(fn SetArmor
  (Variables|Stats|SetArmor (+ (Variables|Basic|GetBasicArmor) (* (Variables|Stats|GetDexterity) 0.14))))

(fn SetMagicResistance
  (Variables|Stats|SetMagicResistance (+ (Variables|Basic|GetBasicMagicResistance) (* (Variables|Stats|GetIntelligence) 0.01))))

(fn LevelUp
  (Variables|Stats|SetPower (+ (Variables|Stats|GetPower) (Variables|LevelGain|GetPowerPerLevelGain)))
  (Variables|Stats|SetDexterity (+ (Variables|Stats|GetDexterity) (Variables|LevelGain|GetDexterityPerLevelGain)))
  (Variables|Stats|SetIntelligence (+ (Variables|Stats|GetIntelligence) (Variables|LevelGain|GetIntelligencePerLevelGain)))
  (Variables|LevelGain|SetLevelPoints (+ (Variables|LevelGain|GetLevelPoints) 1))
  (CallFunction|RecheckCharacteristics))

(fn RecheckCharacteristics
  (CallFunction|SetStats)
  (CallFunction|SetMaxHeath)
  (CallFunction|SetAttack)
  (CallFunction|SetAttackSpeed)
  (CallFunction|SetRegenHeath)
  (CallFunction|SetMaxMana)
  (CallFunction|SetArmor)
  (CallFunction|SetRegenMana)
  (CallFunction|SetMagicResistance)
  (bind _asbp_player (Utilities|Casting|CastToBP_Player (Game|Player|GetPlayerPawn 0)))
  (Variables|/Game/Systems/BPC_DamageSystem.BPC_DamageSystem_C|SetMaxHealth (Variables|/Game/Systems/Player/BP_Player.BP_Player_C|GetBPC_DamageSystem _asbp_player) (Variables|Health|GetMaxHealth)))

(fn SetAttackSpeed
  (Variables|Attack|SetAttackSpeed (/ 1.0 (/ (/ (Variables|Basic|GetBaseAttackSpeed) 1e+02) (Variables|Basic|GetBaseAttackTime)))))

(fn SetStats
  (Variables|Basic|SetStatsInArray (Utilities|Array|MakeArray (Variables|Stats|GetPower) (Variables|Stats|GetDexterity) (Variables|Stats|GetIntelligence))))
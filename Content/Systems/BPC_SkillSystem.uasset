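; Skill component that offers area, cone, projectile and single-target damage functions, plus simple cooldown helpers.
; Area, cone and projectile skills spawn helper actors and bind to their overlap or impact events, while targeted damage hits and clears player 0's CurrentTarget.
; DoDamage sends a TakeDamageMessage with the owner as attacker, using one stored DamageInfo that each skill call overwrites.
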(event Custom|Hit
  (params (OtherActor :type Actor%20Object%20Reference) (Hit :type Hit%20Result%20Structure))
  (CallFunction|DoDamage OtherActor))

(event Custom|DoDamage
  (params (Actor :type Actor%20Object%20Reference))
  (bind _wasdamaged (Class|BPIDamagalbe|TakeDamage(Message) Actor (Variables|Default|GetDamageInfo) (Components|GetOwner)))
  (Development|PrintString (Utilities|String|ToString(Boolean) _wasdamaged)))

(event EventBeginPlay)

(event EventTick
  (params (DeltaSeconds :type Float%20%28single-precision%29)))

(fn AoeDamage
  (params (DamageInfo :type S%20Damage%20Info%20Structure) (Location :type Vector) (Owner :type Pawn%20Object%20Reference) (Radius :type Float%20%28double-precision%29) (Delay :type Float%20%28double-precision%29) (IgnoreInstigator :type Boolean) (DrawDebug :type Boolean))
  (bind (_x _y _z) (Math|Vector|BreakVector Location))
  (Variables|Default|SetDamageInfo DamageInfo)
  (bind _returnvalue (Game|SpawnActorfromClass "/Game/AOE/BP_Aoe_Damage.BP_Aoe_Damage_C" (Math|Transform|MakeTransform (Math|Vector|MakeVector _x _y (+ _z Radius)) "0, 0, 0" "1.000000,1.000000,1.000000") "Undefined" "MultiplyWithRoot" Owner Radius IgnoreInstigator DrawDebug Delay Owner))
  (EventDispatchers|BindEventtoOnAoeOverlapActor _returnvalue (EventDispatchers|CreateEvent :!event Custom|DoDamage)))

(fn TargetDamage
  (params (DamageInfo :type S%20Damage%20Info%20Structure))
  (Variables|Default|SetDamageInfo DamageInfo)
  (bind _asbp_top_down_controller (Utilities|Casting|CastToBP_TopDownController (Game|GetPlayerController 0)))
  (Utilities|IsValid (Variables|/Game/TopDown/Blueprints/BP_TopDownController.BP_TopDownController_C|GetCurrentTarget _asbp_top_down_controller)
    (:Is%20Valid
      (Development|PrintString (Utilities|String|ToString(Object) (Variables|/Game/TopDown/Blueprints/BP_TopDownController.BP_TopDownController_C|GetCurrentTarget _asbp_top_down_controller)))
      (CallFunction|DoDamage (Variables|/Game/TopDown/Blueprints/BP_TopDownController.BP_TopDownController_C|GetCurrentTarget _asbp_top_down_controller))
      (Variables|/Game/TopDown/Blueprints/BP_TopDownController.BP_TopDownController_C|SetCurrentTarget _asbp_top_down_controller 0)
      (return true))
    (:Is%20Not%20Valid
      (return false))))

(fn ProjectileDamage
  (params (DamageInfo :type S%20Damage%20Info%20Structure) (SpawnLocation :type Vector) (TargetLocation :type Vector) (Owner :type Pawn%20Object%20Reference) (Speed :type Float%20%28double-precision%29) (IsHoming :type Boolean) (Target :type Actor%20Object%20Reference) (ActorsToIgnore :type Array%20of%20Actor%20Object%20References))
  (Variables|Default|SetDamageInfo DamageInfo)
  (bind _returnvalue (Game|SpawnActorfromClass "/Game/Systems/Projectiles/BP_Projectile_Skill.BP_Projectile_Skill_C" (Math|Transform|MakeTransform SpawnLocation "0, 0, 0" "1.000000,1.000000,1.000000") "Undefined" "MultiplyWithRoot" Owner Speed "/Game/StarterContent/Particles/P_Smoke.P_Smoke" "/Game/Systems/AudioPlayer/способность-бросок-камня-попадание.способность-бросок-камня-попадание" Target IsHoming TargetLocation ActorsToIgnore Owner))
  (EventDispatchers|BindEventtoOnProjectileImpact _returnvalue (EventDispatchers|CreateEvent :!event Custom|Hit))
  (return _returnvalue))

(fn CheckCooldown
  (params (SkillCooldown :type Float%20%28double-precision%29) (TargetCooldown :type Float%20%28double-precision%29))
  (return (< SkillCooldown TargetCooldown)))

(fn CountCooldown
  (params (Cooldown :type Float%20%28double-precision%29) (Delta :type Float%20%28double-precision%29))
  (return (+ Cooldown Delta)))

(fn ConeDamage
  (params (DamageInfo :type S%20Damage%20Info%20Structure) (Location :type Vector) (Owner :type Pawn%20Object%20Reference) (Angle :type Float%20%28double-precision%29) (Length :type Float%20%28double-precision%29) (Delay :type Float%20%28double-precision%29) (DrawDebug :type Boolean))
  (bind _returnvalue (Transformation|GetActorForwardVector Owner))
  (Variables|Default|SetDamageInfo DamageInfo)
  (bind _returnvalue_2 (Game|SpawnActorfromClass "/Game/AOE/BP_Cone_base.BP_Cone_base_C" (Math|Transform|MakeTransform (+ Location _returnvalue) (Math|Conversions|RotationFromXVector _returnvalue) (Math|Vector|MakeVector 1.0 1.0 1.0)) "AlwaysSpawn" "MultiplyWithRoot" Owner Angle Delay Length true DrawDebug Owner))
  (EventDispatchers|BindEventtoOnConeOverlapActor _returnvalue_2 (EventDispatchers|CreateEvent :!event Custom|DoDamage)))
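; Test enemy creep that fights through shared characteristics, damage and auto-attack components, with a health bar widget and debug attack-range circle.
; A looping timer scales its health, damage and kill gold from per-level creep stats.
; Damage responses switch its AI controller to attack the latest attacker.
; On death it pays gold to that attacker if it is BP_Player, then enables physics and immediately destroys itself.
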(event Custom|Upgrade
  (bind _bpc_characteristics (Variables|Default|GetBPC_Characteristics))
  (bind _bpc_creepstats (Variables|Default|GetBPC_CreepStats))
  (bind _basicattack (Variables|/Game/Systems/BPC_Characteristics.BPC_Characteristics_C|GetBasicAttack _bpc_characteristics))
  (bind _killgold (Variables|/Game/Systems/BPC_CreepStats.BPC_CreepStats_C|GetKillGold _bpc_creepstats))
  (Variables|/Game/Systems/BPC_Characteristics.BPC_Characteristics_C|SetBasicHealth _bpc_characteristics (+ (Variables|/Game/Systems/BPC_Characteristics.BPC_Characteristics_C|GetBasicHealth _bpc_characteristics) (Variables|/Game/Systems/BPC_CreepStats.BPC_CreepStats_C|GetHealthPerLevel _bpc_creepstats)))
  (for (_array_element _array_index) _basicattack
    (Utilities|Array|SetArrayElem _basicattack _array_index (+ _array_element (Variables|/Game/Systems/BPC_CreepStats.BPC_CreepStats_C|GetDamagePerLevel _bpc_creepstats))))
  (for (_array_element_2 _array_index_2) _killgold
    (Utilities|Array|SetArrayElem _killgold _array_index_2 (+ _array_element_2 (Variables|/Game/Systems/BPC_CreepStats.BPC_CreepStats_C|GetGoldPerLevel _bpc_creepstats)))))

(event Custom|Attack
  (params (Target :type Actor%20Object%20Reference))
  (bind _bpc_autoattack (Variables|Default|GetBPC_AutoAttack))
  (bind _bpc_characteristics (Variables|Default|GetBPC_Characteristics))
  (if (not (Variables|/Game/Systems/BPC_DamageSystem.BPC_DamageSystem_C|GetIsDead (Variables|Default|GetBPC_DamageSystem)))
    (Variables|/Game/Systems/BPC_AutoAttack.BPC_AutoAttack_C|SetTarget _bpc_autoattack Target)
    (Default|Attack _bpc_autoattack (Variables|/Game/Systems/BPC_Characteristics.BPC_Characteristics_C|GetAttack _bpc_characteristics) (Variables|/Game/Systems/BPC_Characteristics.BPC_Characteristics_C|GetAttackRange _bpc_characteristics) (Variables|/Game/Systems/BPC_Characteristics.BPC_Characteristics_C|GetCritChance _bpc_characteristics) (Variables|/Game/Systems/BPC_Characteristics.BPC_Characteristics_C|GetCritMultiplier _bpc_characteristics) (Variables|/Game/Systems/BPC_DamageSystem.BPC_DamageSystem_C|GetResponce (Variables|Default|GetBPC_DamageSystem)) (Utilities|Time|GetWorldDeltaSeconds))))

(event Custom|OnDeath
  (bind _mesh (Variables|Character|GetMesh))
  (bind _bpc_damagesystem (Variables|Default|GetBPC_DamageSystem))
  (bind _attackerinfo (Variables|/Game/Systems/BPC_DamageSystem.BPC_DamageSystem_C|GetAttackerInfo _bpc_damagesystem))
  (bind _asbp_player (Utilities|Casting|CastToBP_Player (.Attacker (Utilities|Struct|BreakS_AttackerInfo (Utilities|Array|Get(acopy) _attackerinfo (Utilities|Array|LastIndex _attackerinfo))))))
  (bind _gold (Default|GetGold (Variables|Default|GetBPC_CreepStats)))
  (Variables|/Game/Systems/Player/BP_Player.BP_Player_C|SetGold _asbp_player (+ (Variables|/Game/Systems/Player/BP_Player.BP_Player_C|GetGold _asbp_player) _gold))
  (Physics|SetSimulatePhysics _mesh true)
  (Collision|SetCollisionEnabled _mesh "QueryAndPhysics")
  (Actor|DestroyActor))

(event Custom|OnHit
  (params (DamageResponse :type E_DamageResponse%20Enum :default "NewEnumerator0"))
  (bind _bpc_damagesystem (Variables|Default|GetBPC_DamageSystem))
  (bind _attackerinfo (Variables|/Game/Systems/BPC_DamageSystem.BPC_DamageSystem_C|GetAttackerInfo _bpc_damagesystem))
  (bind _asaic_enemy_base (Utilities|Casting|CastToAIC_Enemy_base (AI|GetAIController self)))
  (Default|SetAttackingState _asaic_enemy_base (.Attacker (Utilities|Struct|BreakS_AttackerInfo (Utilities|Array|Get(acopy) _attackerinfo (Utilities|Array|LastIndex _attackerinfo)))))
  (Development|PrintString (Utilities|String|EnumtoString DamageResponse)))

(event Custom|SetMaxHealth_1
  (params (NewMaxHealth :type Float%20%28double-precision%29)))

(event EventBeginPlay
  (Utilities|FlowControl|Sequence
    (:then_0
      (Utilities|Time|SetTimerbyEvent (delegate Custom|Upgrade) (Variables|Default|GetUpgradeTimeInSeconds) true))
    (:then_1
      (bind _returnvalue (UserInterface|CreateWidget "/Game/Systems/W_HealthBar.W_HealthBar_C" 0 self))
      (UserInterface|SetWidget (Variables|Default|GetHealth) _returnvalue))
    (:then_2
      (Variables|/Game/Systems/BPC_AutoAttack.BPC_AutoAttack_C|SetAttackCooldown (Variables|Default|GetBPC_AutoAttack) 1e+02))))

(event MouseInput|EventActorOnClicked
  (params (ButtonPressed :type Key%20Structure :default "None")))

(event EventTick
  (params (DeltaSeconds :type Float%20%28single-precision%29))
  (Rendering|Debug|DrawDebugCircle (Transformation|GetActorLocation) (Variables|/Game/Systems/BPC_Characteristics.BPC_Characteristics_C|GetAttackRange (Variables|Default|GetBPC_Characteristics)) 12 "(R=1.000000,G=0.000000,B=0.198145,A=1.000000)" 0.0 2.0 "0.000000,1.000000,0.000000" "1.000000,0.000000,0.000000" true))

(fn ConstructionScript
  (bind _bpc_damagesystem (Variables|Default|GetBPC_DamageSystem))
  (EventDispatchers|BindEventtoOnDeath _bpc_damagesystem (EventDispatchers|CreateEvent :!event Custom|OnDeath))
  (EventDispatchers|BindEventtoOnDamageResponse _bpc_damagesystem (EventDispatchers|CreateEvent :!event Custom|OnHit)))

(fn GetAttackSpeed
  (bind _attacksinsecnod (Default|GetAttackSpeed (Variables|Default|GetBPC_Characteristics)))
  (return _attacksinsecnod))

(fn GetCurrentHealth
  (return (Variables|/Game/Systems/BPC_DamageSystem.BPC_DamageSystem_C|GetHealth (Variables|Default|GetBPC_DamageSystem))))

(fn GetCurrentMana
  (return 0.0))

(fn GetMaxHealth
  (return (Variables|/Game/Systems/BPC_DamageSystem.BPC_DamageSystem_C|GetMaxHealth (Variables|Default|GetBPC_DamageSystem))))

(fn GetMaxMana
  (return 0.0))

(fn Heal
  (params (Amount :type Float%20%28double-precision%29))
  (bind _newhealth (Default|Heal (Variables|Default|GetBPC_DamageSystem) Amount))
  (return _newhealth))

(fn TakeDamage
  (params (DamageInfo :type S%20Damage%20Info%20Structure) (Attacker :type Actor%20Object%20Reference))
  (bind _bpc_characteristics (Variables|Default|GetBPC_Characteristics))
  (bind _wasdamaged (Default|TakeDamage (Variables|Default|GetBPC_DamageSystem) DamageInfo (Variables|/Game/Systems/BPC_Characteristics.BPC_Characteristics_C|GetArmor _bpc_characteristics) (Variables|/Game/Systems/BPC_Characteristics.BPC_Characteristics_C|GetMagicResistance _bpc_characteristics) (Variables|Default|GetHasMagicInvulnerability) Attacker))
  (return _wasdamaged))
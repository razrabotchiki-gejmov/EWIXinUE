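; Melee creep enemy with two timed skills that grants XP to the last attacking player on death.
; Skill 1 temporarily boosts armor and attack speed, with a timed cooldown.
; Skill 2 hides the mesh at half health or below, then randomly grants guaranteed crits briefly or boosts regen and sends the AI into its returning state.
; Hits restore visibility and base regen; Skill 2's cooldown flag is never reset here.
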(event Custom|Activate1Skill
  (bind _bpc_characteristics (Variables|Default|GetBPC_Characteristics))
  (if (not (Variables|Default|GetSkill1OnCooldown))
    (Variables|/Game/Systems/BPC_Characteristics.BPC_Characteristics_C|SetArmor _bpc_characteristics (+ (Variables|/Game/Systems/BPC_Characteristics.BPC_Characteristics_C|GetArmor _bpc_characteristics) (Variables|Default|GetSkill1ArmorIncrease)))
    (Default|AddAttackSpeed _bpc_characteristics (Variables|Default|GetSkill1AttackSpeedIncrease))
    (Utilities|Time|SetTimerbyEvent (delegate Custom|EffectEnd) (Variables|Default|GetSkill1EffectTime))
    (Variables|Default|SetSkill1OnCooldown true)
    (Utilities|Time|SetTimerbyEvent (delegate Custom|SetSkill1Cooldown) (Variables|Default|GetSkill1Cooldown))))

(event Custom|EffectEnd
  (bind _bpc_characteristics (Variables|Default|GetBPC_Characteristics))
  (Variables|/Game/Systems/BPC_Characteristics.BPC_Characteristics_C|SetArmor _bpc_characteristics (- (Variables|/Game/Systems/BPC_Characteristics.BPC_Characteristics_C|GetArmor _bpc_characteristics) (Variables|Default|GetSkill1ArmorIncrease)))
  (Default|AddAttackSpeed _bpc_characteristics (* (Variables|Default|GetSkill1AttackSpeedIncrease) -1.0)))

(event Custom|SetSkill1Cooldown
  (Variables|Default|SetSkill1OnCooldown false))

(event Custom|Activate2Skill
  (bind _bpc_characteristics (Variables|Default|GetBPC_Characteristics))
  (if (not (Variables|Default|GetSkill2OnCooldown))
    (if (<= (Variables|/Game/Systems/BPC_DamageSystem.BPC_DamageSystem_C|GetHealth (Variables|Default|GetBPC_DamageSystem)) (/ (Variables|/Game/Systems/BPC_Characteristics.BPC_Characteristics_C|GetMaxHealth (Variables|Default|GetBPC_Characteristics)) 2.0))
      (Rendering|SetVisibility (Variables|Character|GetMesh) false false)
      (if (>= (Math|Random|RandomFloat) 0.5)
        (Variables|/Game/Systems/BPC_Characteristics.BPC_Characteristics_C|SetCritChance (Variables|Default|GetBPC_Characteristics) 1e+02)
        (Utilities|Time|SetTimerbyEvent (delegate Custom|DecreaseCritChance) 1.5)
        (Variables|Default|SetSkill2OnCooldown true)
        (else
          (Variables|/Game/Systems/BPC_Characteristics.BPC_Characteristics_C|SetRegenHealth _bpc_characteristics (+ (Variables|/Game/Systems/BPC_Characteristics.BPC_Characteristics_C|GetBasicRegenHealth _bpc_characteristics) (Variables|Default|GetSkill2HealthRegen)))
          (Utilities|Time|SetTimerbyEvent (delegate Custom|EndInvisibility) (Variables|Default|GetSkill2EffectTime))
          (Variables|Default|SetSkill2OnCooldown true)
          (bind _asaic_enemy_base (Utilities|Casting|CastToAIC_Enemy_base (AI|GetAIController self)))
          (Default|SetReturningState _asaic_enemy_base))))))

(event Custom|EndInvisibility
  (bind _bpc_characteristics (Variables|Default|GetBPC_Characteristics))
  (Rendering|SetVisibility (Variables|Character|GetMesh) true false)
  (Variables|/Game/Systems/BPC_Characteristics.BPC_Characteristics_C|SetRegenHealth _bpc_characteristics (Variables|/Game/Systems/BPC_Characteristics.BPC_Characteristics_C|GetBasicRegenHealth _bpc_characteristics)))

(event Custom|DecreaseCritChance
  (Variables|/Game/Systems/BPC_Characteristics.BPC_Characteristics_C|SetCritChance (Variables|Default|GetBPC_Characteristics) 0.0))

(event EventBeginPlay
  (|CallParentFunction) ; This node is disabled and will not be called.\nDrag off pins to build functionality.
)

(event Collision|EventActorBeginOverlap
  (params (OtherActor :type Actor%20Object%20Reference)))

(event EventTick
  (params (DeltaSeconds :type Float%20%28single-precision%29))
  (|CallParentFunction DeltaSeconds) ; This node is disabled and will not be called.\nDrag off pins to build functionality.
)

(event EventOnDeath
  (bind _bpc_characteristics (Variables|Default|GetBPC_Characteristics))
  (bind _bpc_damagesystem (Variables|Default|GetBPC_DamageSystem))
  (bind _attackerinfo (Variables|/Game/Systems/BPC_DamageSystem.BPC_DamageSystem_C|GetAttackerInfo _bpc_damagesystem))
  (|CallParentFunction)
  (bind _experienceforkill (Default|GetXPforKillforCreep _bpc_characteristics (Variables|/Game/Systems/BPC_Characteristics.BPC_Characteristics_C|GetLevel _bpc_characteristics)))
  (bind _asbp_player (Utilities|Casting|CastToBP_Player (.Attacker (Utilities|Struct|BreakS_AttackerInfo (Utilities|Array|Get(acopy) _attackerinfo (Utilities|Array|LastIndex _attackerinfo))))))
  (Default|OnExpGet _asbp_player _experienceforkill)
  (Actor|DestroyActor))

(event EventOnHit
  (params (DamageResponse :type E_DamageResponse%20Enum :default "NewEnumerator0"))
  (bind _bpc_characteristics (Variables|Default|GetBPC_Characteristics))
  (|CallParentFunction DamageResponse)
  (Rendering|SetVisibility (Variables|Character|GetMesh) true false)
  (Variables|/Game/Systems/BPC_Characteristics.BPC_Characteristics_C|SetRegenHealth _bpc_characteristics (Variables|/Game/Systems/BPC_Characteristics.BPC_Characteristics_C|GetBasicRegenHealth _bpc_characteristics)))

(event EventSetCharaterMaxHeath)

(fn ConstructionScript
  (|CallParentFunction))
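; Mega melee creep enemy with two targeted skills that awards hero-boss-tier XP to its last attacker, if a player, on death.
; Skill 1 drains mana from an in-range target on a repeating timer, healing the creep for half, then pauses into cooldown after a capped tick count.
; Skill 2 fires a projectile that ignores camp members, then deals AoE damage and starts its cooldown when the projectile is destroyed.
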(event Custom|Skill1Activation
  (params (Target :type Actor%20Object%20Reference))
  (if (not (Variables|Default|GetSkill1OnCooldown))
    (bind _output_get (Variables|Default|SetSkill1TargetInRange (<= (Math|Float|Absolute(Float) (Math|Vector|VectorLength (- (Transformation|GetActorLocation Target) (Transformation|GetActorLocation self)))) (Variables|Default|GetSkill1Range))))
    (if _output_get
      (if (not (Variables|Default|GetSkill1IsActive))
        (Variables|Default|SetSkill1OnCooldown true)
        (Utilities|Time|SetTimerbyEvent (delegate Custom|ManaDrain) 0.0)
        (bind _returnvalue (Utilities|Time|SetTimerbyEvent (delegate Custom|ManaDrain) 1.0 true))))))

(event Custom|ManaDrain
  (if (<= (Math|Float|Absolute(Float) (Math|Vector|VectorLength (- (Transformation|GetActorLocation (stale Custom|Skill1Activation Target)) (Transformation|GetActorLocation self)))) (Variables|Default|GetSkill1Range))
    (Variables|Default|SetSkill1IsActive true)
    (bind _output_get (Variables|Default|SetSkill1Counts (+ (Variables|Default|GetSkill1Counts) 1.0)))
    (if (>= _output_get 1e+01)
      (Utilities|Time|PauseTimerbyHandle (stale Custom|Skill1Activation _returnvalue))
      (Utilities|Time|SetTimerbyEvent (delegate Custom|Skill1Cooldown) 6e+01)
      (elif (> (Variables|/Game/Systems/BPC_Characteristics.BPC_Characteristics_C|GetMana (Actor|GetComponentbyClass (stale Custom|Skill1Activation Target) "/Game/Systems/BPC_Characteristics.BPC_Characteristics_C")) 0.0)
        (CallFunction|Heal (/ (- (Variables|/Game/Systems/BPC_Characteristics.BPC_Characteristics_C|GetMana (Actor|GetComponentbyClass (stale Custom|Skill1Activation Target) "/Game/Systems/BPC_Characteristics.BPC_Characteristics_C")) (Math|Float|Clamp(Float) (- (Variables|/Game/Systems/BPC_Characteristics.BPC_Characteristics_C|GetMana (Actor|GetComponentbyClass (stale Custom|Skill1Activation Target) "/Game/Systems/BPC_Characteristics.BPC_Characteristics_C")) 5.0) 0.0 (Variables|/Game/Systems/BPC_Characteristics.BPC_Characteristics_C|GetMaxMana (Actor|GetComponentbyClass (stale Custom|Skill1Activation Target) "/Game/Systems/BPC_Characteristics.BPC_Characteristics_C")))) 2.0))
        (Variables|/Game/Systems/BPC_Characteristics.BPC_Characteristics_C|SetMana (Actor|GetComponentbyClass (stale Custom|Skill1Activation Target) "/Game/Systems/BPC_Characteristics.BPC_Characteristics_C") (Math|Float|Clamp(Float) (- (Variables|/Game/Systems/BPC_Characteristics.BPC_Characteristics_C|GetMana (Actor|GetComponentbyClass (stale Custom|Skill1Activation Target) "/Game/Systems/BPC_Characteristics.BPC_Characteristics_C")) 5.0) 0.0 (Variables|/Game/Systems/BPC_Characteristics.BPC_Characteristics_C|GetMaxMana (Actor|GetComponentbyClass (stale Custom|Skill1Activation Target) "/Game/Systems/BPC_Characteristics.BPC_Characteristics_C"))))))
    (else
      (Variables|Default|SetSkill1Counts (+ (Variables|Default|GetSkill1Counts) 1.0)))))

(event Custom|Skill1Cooldown
  (Variables|Default|SetSkill1OnCooldown false))

(event Custom|Skill2Activation
  (params (Target :type Actor%20Object%20Reference))
  (bind _returnvalue (Transformation|GetActorLocation Target))
  (bind _self self)
  (if (not (Variables|Default|GetSkill2OnCooldown))
    (if (<= (Math|Float|Absolute(Float) (Math|Vector|VectorLength (- _returnvalue (Transformation|GetActorLocation self)))) (.Range (Utilities|Struct|BreakS_SkillInfo (Variables|Default|GetSkill2Info))))
      (bind _actors (Class|BPICamp|GetSpawnedActors(Message) (Variables|Default|GetCamp)))
      (bind _projectiletoignore (Default|ProjectileDamage :self (Variables|Default|GetBPC_SkillSystem) :SpawnLocation (Transformation|GetActorLocation _self) :TargetLocation _returnvalue :Owner _self :Speed (Variables|Default|GetSkill2ProjectileSpeed) :Target Target :ActorsToIgnore _actors))
      (Variables|Default|SetSkill2OnCooldown true)
      (bind _actors_2 (Class|BPICamp|GetSpawnedActors(Message) (Variables|Default|GetCamp)))
      (for _array_element _actors_2
        (bind _mesh (Class|BPICharacter|GetMesh(Message) _array_element))
        (Collision|IgnoreActorwhenMoving _mesh _projectiletoignore true))
      (Game|AssignOnDestroyed _projectiletoignore (delegate Custom|OnDestroy)))))

(event Custom|Skill2Cooldown
  (Variables|Default|SetSkill2OnCooldown false))

(event Custom|OnDestroy
  (params (DestroyedActor :type Actor%20Object%20Reference))
  (bind _skill2info (Variables|Default|GetSkill2Info))
  (bind (_damage _manacost _cooldown _range) (Utilities|Struct|BreakS_SkillInfo _skill2info))
  (Default|AoeDamage (Variables|Default|GetBPC_SkillSystem) _damage (Transformation|GetActorLocation (stale Custom|Skill2Activation _projectiletoignore)) self (Variables|Default|GetSkill2SphereRange) 0.0 true false)
  (Utilities|Time|SetTimerbyEvent (delegate Custom|Skill2Cooldown) _cooldown))

(event EventBeginPlay
  (|CallParentFunction) ; This node is disabled and will not be called.\nDrag off pins to build functionality.
)

(event Collision|EventActorBeginOverlap
  (params (OtherActor :type Actor%20Object%20Reference)))

(event EventTick
  (params (DeltaSeconds :type Float%20%28single-precision%29))
  (|CallParentFunction DeltaSeconds) ; This node is disabled and will not be called.\nDrag off pins to build functionality.
)

(event EventOnDeath
  (bind _bpc_characteristics (Variables|Default|GetBPC_Characteristics))
  (bind _bpc_damagesystem (Variables|Default|GetBPC_DamageSystem))
  (bind _attackerinfo (Variables|/Game/Systems/BPC_DamageSystem.BPC_DamageSystem_C|GetAttackerInfo _bpc_damagesystem))
  (|CallParentFunction)
  (bind _experienceforkill (Default|GetXPforKillforHeroBoss _bpc_characteristics (Variables|/Game/Systems/BPC_Characteristics.BPC_Characteristics_C|GetLevel _bpc_characteristics)))
  (bind _asbp_player (Utilities|Casting|CastToBP_Player (.Attacker (Utilities|Struct|BreakS_AttackerInfo (Utilities|Array|Get(acopy) _attackerinfo (Utilities|Array|LastIndex _attackerinfo))))))
  (Default|OnExpGet _asbp_player _experienceforkill)
  (Actor|DestroyActor))

(fn ConstructionScript
  (|CallParentFunction))

(fn GetAttackSpeed
  (bind _attacksinsecnod (Default|GetAttackSpeed (Variables|Default|GetBPC_Characteristics)))
  (return _attacksinsecnod))
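; Base actor for an enemy creep camp that respawns and strengthens its creeps over time.
; A looping timer spawns every class in Creeps when no actors overlap the camp, applying start-level upgrades plus time upgrades from UpgradeCount.
; A second timer upgrades spawned creeps, incrementing UpgradeCount per creep rather than per tick.
; SetAttackerForCreepsInCamp shares an attacker with the camp's creeps through their AI controllers.
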(event Custom|SpawnEnemy
  (bind _upgradecount (Variables|Upgrade|GetUpgradeCount))
  (bind _spawnedcreeps (Variables|Creeps|GetSpawnedCreeps))
  (bind _returnvalue (- _upgradecount 1.0))
  (if (Variables|Default|GetCampEmpty)
    (for _array_element (Variables|Creeps|GetCreeps)
      (bind _returnvalue_2 (Game|SpawnActorfromClass _array_element (Transformation|GetActorTransform) "AdjustIfPossibleButAlwaysSpawn" "MultiplyWithRoot" 0 0))
      (Utilities|Array|SetArrayElem _spawnedcreeps (+ (Utilities|Array|LastIndex _spawnedcreeps) 1) _returnvalue_2 true)
      (bind _asbp_enemy_ai_base (Utilities|Casting|CastToBP_Enemy_AI_Base _returnvalue_2))
      (Variables|/Game/Systems/Enemy/Creeps/BP_Enemy_AI_Base.BP_Enemy_AI_Base_C|SetCamp _asbp_enemy_ai_base self)
      (for _index (range 0 (- (Math|Float|Truncate (Variables|Upgrade|GetStartLevelOfCreeps)) 1))
        (Default|UpgradeonSpawn _asbp_enemy_ai_base))
      (if (>= _returnvalue 0.0)
        (for _index_2 (range 0 (Math|Float|Truncate _returnvalue))
          (Default|UpgradebyTime _asbp_enemy_ai_base))))))

(event Custom|OnActorBeginOverlap_Event
  (params (OverlappedActor :type Actor%20Object%20Reference) (OtherActor :type Actor%20Object%20Reference))
  (bind _overlappedactors (Variables|Default|GetOverlappedActors))
  (Utilities|Array|SetArrayElem _overlappedactors (+ (Utilities|Array|LastIndex _overlappedactors) 1) OtherActor true)
  (CallFunction|CheckifNoCreepsinCamp))

(event Custom|OnActorEndOverlap_Event
  (params (OverlappedActor :type Actor%20Object%20Reference) (OtherActor :type Actor%20Object%20Reference))
  (Utilities|Array|RemoveItem (Variables|Default|GetOverlappedActors) OtherActor)
  (CallFunction|CheckifNoCreepsinCamp))

(event Custom|UpgradeCreeps
  (for _array_element (Variables|Creeps|GetSpawnedCreeps)
    (bind _asbp_enemy_ai_base (Utilities|Casting|CastToBP_Enemy_AI_Base _array_element))
    (if (>= (Math|Float|Floor (/ (Utilities|Time|GetTimeSeconds) (Variables|Upgrade|GetUpgradeTime))) 1)
      (Default|UpgradebyTime _asbp_enemy_ai_base)
      (Variables|Upgrade|SetUpgradeCount (+ (Variables|Upgrade|GetUpgradeCount) 1.0)))))

(event Custom|SetAttackerForCreepsInCamp
  (params (Attacker :type Actor%20Object%20Reference))
  (for _array_element (Variables|Creeps|GetSpawnedCreeps)
    (bind _asbp_enemy_ai_base (Utilities|Casting|CastToBP_Enemy_AI_Base _array_element))
    (bind _asaic_enemy_base (Utilities|Casting|CastToAIC_Enemy_base (AI|GetAIController _asbp_enemy_ai_base)))
    (Default|SetAttackingState _asaic_enemy_base Attacker)))

(event Custom|CheckIfNoCreepsInCamp
  (if (>= (Utilities|Array|Length (Variables|Default|GetOverlappedActors)) 1)
    (Variables|Default|SetCampEmpty false)
    (else
      (Variables|Default|SetCampEmpty true))))

(event EventBeginPlay
  (EventDispatchers|BindEventtoOnActorBeginOverlap (delegate Custom|OnActorBeginOverlap_Event))
  (EventDispatchers|BindEventtoOnActorEndOverlap (delegate Custom|OnActorEndOverlap_Event))
  (Utilities|Time|SetTimerbyEvent (delegate Custom|SpawnEnemy) (Variables|SpawnTime|GetRespawnTime) true)
  (Utilities|Time|SetTimerbyEvent (delegate Custom|UpgradeCreeps) (Variables|Upgrade|GetUpgradeTime) true))

(fn ConstructionScript)

(fn GetSpawnedActors
  (return (Variables|Creeps|GetSpawnedCreeps)))
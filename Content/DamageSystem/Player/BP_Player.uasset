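; Player character Blueprint with a health bar, three click-cast area skills, ragdoll on death and debug prints for hits.
; Q, W or E arms a skill; left click spawns its AoE actor, with damage and explosion at the cursor hit and heal at the player.
; Each AoE's overlap event sends damage or heal messages to overlapped actors.
; The player's own damage, heal and health queries forward to BPCDamageSystem, whose death and response events are bound in construction.
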(event Custom|DealDamageAOE
  (params (Actor :type Actor%20Object%20Reference))
  (bind _wasdamaged (Class|BPIDamagalbe|TakeDamage(Message) Actor (Utilities|Struct|MakeS_DamageInfo 15.0 "NewEnumerator1" "NewEnumerator1")))
  (Development|PrintString (Utilities|String|ToString(Boolean) _wasdamaged)))

(event Custom|OnDeath
  (bind _mesh (Variables|Character|GetMesh))
  (Physics|SetSimulatePhysics _mesh true)
  (Collision|SetCollisionEnabled _mesh "QueryAndPhysics")
  (Input|DisableInput (Game|GetPlayerController 0)))

(event Custom|OnHit
  (params (DamageResponse :type E_DamageResponse%20Enum :default "NewEnumerator0"))
  (Development|PrintString (Utilities|String|EnumtoString DamageResponse)))

(event Custom|HealSkillAOE
  (params (Actor :type Actor%20Object%20Reference))
  (Class|BPIDamagalbe|Heal(Message) Actor 1e+01))

(event Custom|DealDamagePoint
  (params (Actor :type Actor%20Object%20Reference))
  (bind _wasdamaged (Class|BPIDamagalbe|TakeDamage(Message) Actor (Utilities|Struct|MakeS_DamageInfo 2e+01 "NewEnumerator1" "NewEnumerator1")))
  (Development|PrintString (Utilities|String|ToString(Boolean) _wasdamaged)))

(event EventBeginPlay
  (Utilities|FlowControl|Sequence
    (:then_1
      (bind _returnvalue (UserInterface|CreateWidget "/Game/DamageSystem/W_HealthBar.W_HealthBar_C" 0 self))
      (UserInterface|SetWidget (Variables|Default|GetHealth) _returnvalue))))

(event Input|KeyboardEvents|Q
  (params (Key :type Key%20Structure :default "None"))
  (:Pressed
    (bind _output_get (Variables|Default|Setskill_activate_1 true))))

(event Input|MouseEvents|LeftMouseButton
  (params (Key :type Key%20Structure :default "None"))
  (bind _returnvalue (Game|GetInstigator))
  (bind _returnvalue_2 (Game|GetPlayerController 0))
  (bind _hitresult (Game|Player|GetHitResultUnderCursorbyChannel _returnvalue_2 "TraceTypeQuery1" true))
  (bind _location (Collision|BreakHitResult _hitresult))
  (:Pressed
    (bind _output_get (Variables|Default|Setmouse_point true))
    (if (and (stale Input|KeyboardEvents|Q _output_get) _output_get)
      (Development|PrintString "Skill activated")
      (Development|PrintString (Utilities|String|ToString(Vector) _location))
      (bind _returnvalue_3 (Game|SpawnActorfromClass "/Game/AOE/BP_Aoe_Damage.BP_Aoe_Damage_C" (Math|Transform|MakeTransform _location "0, 0, 0" "1.000000,1.000000,1.000000") "Undefined" "MultiplyWithRoot" _returnvalue 1e+02 true true 0.2 _returnvalue))
      (EventDispatchers|AssignOnAoeOverlapActor _returnvalue_3 (delegate Custom|DealDamageAOE))))
  (:Released
    (Variables|Default|Setmouse_point false)
    (Variables|Default|Setskill_activate_1 false)))

(event Input|KeyboardEvents|W
  (params (Key :type Key%20Structure :default "None"))
  (:Pressed
    (bind _output_get (Variables|Default|Setskill_activate_2 true))))

(event Input|MouseEvents|LeftMouseButton
  (params (Key :type Key%20Structure :default "None"))
  (bind _returnvalue (Game|GetInstigator))
  (bind _returnvalue_2 (Game|GetPlayerController 0))
  (bind _hitresult (Game|Player|GetHitResultUnderCursorbyChannel _returnvalue_2 "TraceTypeQuery1" true))
  (bind _location (Collision|BreakHitResult _hitresult))
  (:Pressed
    (bind _output_get (Variables|Default|Setmouse_point true))
    (if (and (stale Input|KeyboardEvents|W _output_get) _output_get)
      (Development|PrintString "Skill activated")
      (Development|PrintString (Utilities|String|ToString(Vector) _location))
      (bind _returnvalue_3 (Game|SpawnActorfromClass "/Game/AOE/BP_Aoe_explosion.BP_Aoe_explosion_C" (Math|Transform|MakeTransform _location "0, 0, 0" "1.000000,1.000000,1.000000") "Undefined" "MultiplyWithRoot" _returnvalue 1.0 true true 0.2 _returnvalue))
      (EventDispatchers|AssignOnAoeOverlapActor _returnvalue_3 (delegate Custom|DealDamagePoint))))
  (:Released
    (Variables|Default|Setmouse_point false)
    (Variables|Default|Setskill_activate_2 false)))

(event Input|KeyboardEvents|E
  (params (Key :type Key%20Structure :default "None"))
  (:Pressed
    (bind _output_get (Variables|Default|Setskill_activate_3 true))))

(event Input|MouseEvents|LeftMouseButton
  (params (Key :type Key%20Structure :default "None"))
  (bind _returnvalue (Game|GetInstigator))
  (bind _returnvalue_2 (Transformation|GetActorLocation))
  (:Pressed
    (bind _output_get (Variables|Default|Setmouse_point true))
    (if (and (stale Input|KeyboardEvents|E _output_get) _output_get)
      (Development|PrintString "Skill activated")
      (Development|PrintString (Utilities|String|ToString(Vector) _returnvalue_2))
      (bind _returnvalue_3 (Game|SpawnActorfromClass "/Game/AOE/BP_AOE_Heal.BP_AOE_Heal_C" (Math|Transform|MakeTransform _returnvalue_2 "0, 0, 0" "1.000000,1.000000,1.000000") "Undefined" "MultiplyWithRoot" _returnvalue 1e+02 false true 0.2 _returnvalue))
      (EventDispatchers|AssignOnAoeOverlapActor _returnvalue_3 (delegate Custom|HealSkillAOE))))
  (:Released
    (Variables|Default|Setmouse_point false)
    (Variables|Default|Setskill_activate_3 false)))

(fn ConstructionScript
  (bind _bpc_damagesystem (Variables|Default|GetBPC_DamageSystem))
  (EventDispatchers|BindEventtoOnDeath _bpc_damagesystem (EventDispatchers|CreateEvent :!event Custom|OnDeath))
  (EventDispatchers|BindEventtoOnDamageResponse _bpc_damagesystem (EventDispatchers|CreateEvent :!event Custom|OnHit)))

(fn GetCurrentHealth
  (return (Variables|/Game/DamageSystem/BPC_DamageSystem.BPC_DamageSystem_C|GetHealth (Variables|Default|GetBPC_DamageSystem))))

(fn GetMaxHealth
  (return (Variables|/Game/DamageSystem/BPC_DamageSystem.BPC_DamageSystem_C|GetMaxHealth (Variables|Default|GetBPC_DamageSystem))))

(fn Heal
  (params (Amount :type Float%20%28double-precision%29))
  (bind _newhealth (Default|Heal (Variables|Default|GetBPC_DamageSystem) Amount))
  (return _newhealth))

(fn TakeDamage
  (params (DamageInfo :type S%20Damage%20Info%20Structure))
  (bind _wasdamaged (Default|TakeDamage (Variables|Default|GetBPC_DamageSystem) DamageInfo 0.0 0.0))
  (return _wasdamaged))
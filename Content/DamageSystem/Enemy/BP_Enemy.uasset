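; BP_Enemy is a damageable enemy that periodically attacks pawns in front of it and can be click-targeted for player skills.
; A looping timer runs a forward sphere trace, sends damage through a message call and spawns an explosion when it succeeds.
; Health, healing and damage delegate to BPCDamageSystem, whose events trigger ragdoll death and debug-print hit responses.
; A health bar widget is bound at BeginPlay, and clicks set the controller's target while a skill is active.
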(event Custom|OnDeath
  (bind _mesh (Variables|Character|GetMesh))
  (Physics|SetSimulatePhysics _mesh true)
  (Collision|SetCollisionEnabled _mesh "QueryAndPhysics"))

(event Custom|OnHit
  (params (DamageResponse :type E_DamageResponse%20Enum :default "NewEnumerator0"))
  (Development|PrintString (Utilities|String|EnumtoString DamageResponse)))

(event Custom|Attack
  (bind _returnvalue (Transformation|GetActorLocation))
  (if (not (Variables|/Game/DamageSystem/BPC_DamageSystem.BPC_DamageSystem_C|GetIsDead (Variables|Default|GetBPC_DamageSystem)))
    (bind (_outhit _returnvalue_2) (Collision|SphereTraceForObjects _returnvalue (+ (* (Transformation|GetActorForwardVector) 1e+02) _returnvalue) 2e+01 (Utilities|Array|MakeArray "ObjectTypeQuery3") false 0 "ForDuration"))
    (if _returnvalue_2
      (bind _wasdamaged (Class|BPIDamagalbe|TakeDamage(Message) (.HitActor (Collision|BreakHitResult _outhit)) (Utilities|Struct|MakeS_DamageInfo 1e+01 "NewEnumerator1" "NewEnumerator1")))
      (if _wasdamaged
        (Effects|SpawnEmitteratLocation "/Game/StarterContent/Particles/P_Explosion.P_Explosion" (.Location (Collision|BreakHitResult _outhit)))))))

(event EventBeginPlay
  (Utilities|FlowControl|Sequence
    (:then_1
      (Utilities|Time|SetTimerbyEvent (delegate Custom|Attack) 2.0 true)
      (bind _returnvalue (UserInterface|CreateWidget "/Game/DamageSystem/W_HealthBar.W_HealthBar_C" 0 self))
      (UserInterface|SetWidget (Variables|Default|GetHealth) _returnvalue))))

(event MouseInput|EventActorOnClicked
  (params (ButtonPressed :type Key%20Structure :default "None"))
  (bind _asbp_player (Utilities|Casting|CastToBP_Player (Game|Player|GetPlayerPawn 0)))
  (if (Math|Boolean|ORBoolean (Variables|/Game/DamageSystem/Player/BP_Player.BP_Player_C|Getskill_activate_1 _asbp_player) (Variables|/Game/DamageSystem/Player/BP_Player.BP_Player_C|Getskill_activate_2 _asbp_player) (Variables|/Game/DamageSystem/Player/BP_Player.BP_Player_C|Getskill_activate_3 _asbp_player))
    (bind _asbp_top_down_controller (Utilities|Casting|CastToBP_TopDownController (Game|GetPlayerController 0)))
    (Variables|/Game/TopDown/Blueprints/BP_TopDownController.BP_TopDownController_C|SetCurrentTarget _asbp_top_down_controller self)))

(fn ConstructionScript
  (bind _bpc_damagesystem (Variables|Default|GetBPC_DamageSystem))
  (EventDispatchers|BindEventtoOnDeath _bpc_damagesystem (EventDispatchers|CreateEvent :!event Custom|OnDeath))
  (EventDispatchers|BindEventtoOnDamageResponse _bpc_damagesystem (EventDispatchers|CreateEvent :!event Custom|OnHit)))

(fn GetCurrentHealth
  (return (Variables|/Game/DamageSystem/BPC_DamageSystem.BPC_DamageSystem_C|GetHealth (Variables|Default|GetBPC_DamageSystem))))

(fn GetMaxHealth
  (return (Variables|/Game/DamageSystem/BPC_DamageSystem.BPC_DamageSystem_C|GetMaxHealth (Variables|Default|GetBPC_DamageSystem))))

(fn Heal
  (params (Amount :type Float%20%28double-precision%29))
  (bind _newhealth (Default|Heal (Variables|Default|GetBPC_DamageSystem) Amount))
  (return _newhealth))

(fn TakeDamage
  (params (DamageInfo :type S%20Damage%20Info%20Structure))
  (bind _wasdamaged (Default|TakeDamage (Variables|Default|GetBPC_DamageSystem) DamageInfo))
  (return _wasdamaged))
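; Skill system component that delivers damage as area-of-effect, targeted or projectile skills.
; Each function stores DamageInfo, then spawns an AoE or projectile actor with bound overlap or impact events, or directly damages the player controller's CurrentTarget and clears it.
; All hits funnel into DoDamage, which sends TakeDamageMessage to the victim and prints the result.
; Homing projectiles take their target from the first player controller.
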(event Custom|Hit
  (params (OtherActor :type Actor%20Object%20Reference) (Hit :type Hit%20Result%20Structure))
  (CallFunction|DoDamage OtherActor))

(event Custom|DoDamage
  (params (Actor :type Actor%20Object%20Reference))
  (bind _wasdamaged (Class|BPIDamagalbe|TakeDamage(Message) Actor (Variables|Default|GetDamageInfo)))
  (Development|PrintString (Utilities|String|ToString(Boolean) _wasdamaged)))

(event EventBeginPlay)

(event EventTick
  (params (DeltaSeconds :type Float%20%28single-precision%29)))

(fn AoeDamage
  (params (DamageInfo :type S%20Damage%20Info%20Structure) (Location :type Vector) (Scale :type Vector) (Owner :type Pawn%20Object%20Reference) (Radius :type Float%20%28double-precision%29) (Delay :type Float%20%28double-precision%29) (IgnoreInstigator :type Boolean) (DrawDebug :type Boolean))
  (bind (_x _y _z) (Math|Vector|BreakVector Location))
  (Variables|Default|SetDamageInfo DamageInfo)
  (bind _returnvalue (Game|SpawnActorfromClass "/Game/AOE/BP_Aoe_Damage.BP_Aoe_Damage_C" (Math|Transform|MakeTransform (Math|Vector|MakeVector _x _y (+ _z Radius)) "0, 0, 0" Scale) "Undefined" "MultiplyWithRoot" Owner Radius IgnoreInstigator DrawDebug Delay Owner))
  (EventDispatchers|BindEventtoOnAoeOverlapActor _returnvalue (EventDispatchers|CreateEvent :!event Custom|DoDamage)))

(fn TargetDamage
  (params (DamageInfo :type S%20Damage%20Info%20Structure))
  (Variables|Default|SetDamageInfo DamageInfo)
  (bind _asbp_top_down_controller (Utilities|Casting|CastToBP_TopDownController (Game|GetPlayerController 0)))
  (Development|PrintString (Utilities|String|ToString(Object) (Variables|/Game/TopDown/Blueprints/BP_TopDownController.BP_TopDownController_C|GetCurrentTarget _asbp_top_down_controller)))
  (CallFunction|DoDamage (Variables|/Game/TopDown/Blueprints/BP_TopDownController.BP_TopDownController_C|GetCurrentTarget _asbp_top_down_controller))
  (Variables|/Game/TopDown/Blueprints/BP_TopDownController.BP_TopDownController_C|SetCurrentTarget _asbp_top_down_controller 0))

(fn ProjectileDamage
  (params (DamageInfo :type S%20Damage%20Info%20Structure) (Location :type Vector) (Owner :type Pawn%20Object%20Reference) (Speed :type Float%20%28double-precision%29) (IsHoming :type Boolean))
  (Variables|Default|SetDamageInfo DamageInfo)
  (if IsHoming
    (bind _asbp_top_down_controller (Utilities|Casting|CastToBP_TopDownController (Game|GetPlayerController 0)))
    (bind _currenttarget (Variables|/Game/TopDown/Blueprints/BP_TopDownController.BP_TopDownController_C|GetCurrentTarget _asbp_top_down_controller)
      (:then
        (bind _output_get (Variables|Default|SetTargetInfo _currenttarget)))
      (:else
        _)))
  (bind _returnvalue (Game|SpawnActorfromClass "/Game/DamageSystem/Projectiles/BP_Projectile_Skill.BP_Projectile_Skill_C" (Math|Transform|MakeTransform Location "0, 0, 0" "1.000000,1.000000,1.000000") "Undefined" "MultiplyWithRoot" Owner Speed "/Game/StarterContent/Particles/P_Smoke.P_Smoke" "/Game/StarterContent/Audio/Explosion01.Explosion01" _output_get false Owner))
  (EventDispatchers|BindEventtoOnProjectileImpact _returnvalue (EventDispatchers|CreateEvent :!event Custom|Hit)))
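; BP_Aoe_blast_base is a base actor for area-of-effect blasts, adding visual and audio feedback to its parent's AOE sphere.
; SpawnAOESphere calls the parent implementation, then spawns an optional attached BlastEffect particle system and plays an optional BlastSound at the actor's location.
; The actor destroys itself when the particle system finishes, or after a short delay if no valid effect is set.
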(event Custom|SystemFinished
  (params (PSystem :type Particle%20System%20Component%20Object%20Reference))
  (Actor|DestroyActor))

(event Custom|SpawnBlastEffect
  (bind _blasteffect (Variables|Default|GetBlastEffect)
    (:then
      (bind _returnvalue (Effects|SpawnEmitterAttached _blasteffect (Variables|Default|GetDefaultSceneRoot) "None"))
      (EventDispatchers|AssignOnSystemFinished _returnvalue (delegate Custom|SystemFinished)))
    (:else
      (Utilities|FlowControl|Delay 0.2)
      (Actor|DestroyActor))))

(event Custom|SpawnBlastSound
  (bind _blastsound (Variables|Default|GetBlastSound)
    (:then
      (Audio|PlaySoundatLocation _blastsound (Transformation|GetActorLocation) "0, 0, 0" 1.0 1.0 0.0 0 0 0 0))
    (:else)))

(event EventBeginPlay
  (|CallParentFunction) ; This node is disabled and will not be called.\nDrag off pins to build functionality.
)

(event Collision|EventActorBeginOverlap
  (params (OtherActor :type Actor%20Object%20Reference)))

(event EventTick
  (params (DeltaSeconds :type Float%20%28single-precision%29)))

(event EventSpawnAOESphere
  (params (radius :type Float%20%28double-precision%29))
  (|CallParentFunction radius)
  (CallFunction|SpawnBlastEffect)
  (CallFunction|SpawnBlastSound))

(fn ConstructionScript
  (|CallParentFunction))
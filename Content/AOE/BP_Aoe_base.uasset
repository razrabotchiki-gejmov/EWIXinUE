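; Base area-of-effect actor that waits a set delay on BeginPlay, runs one sphere overlap, then destroys itself.
; The overlap finds Pawns within the radius around the actor, optionally ignoring the instigator and drawing a debug sphere.
; Each hit is broadcast through the OnAoeOverlapActor dispatcher, leaving the effect to listeners, and its name is printed.
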(event Custom|SpawnAOESphere
  (params (radius :type Float%20%28double-precision%29))
  (bind _output_get (Variables|Default|SetRadius radius))
  (if (Variables|Default|GetDrawDebug)
    (Rendering|Debug|DrawDebugSphere (Transformation|GetActorLocation) _output_get 12 "(R=1.000000,G=0.000000,B=0.844682,A=1.000000)" 2.0 1.0))
  (bind _outactors (Collision|SphereOverlapActors (Transformation|GetActorLocation) _output_get (Utilities|Array|MakeArray "ObjectTypeQuery3") 0 (select (Variables|Default|GetIgnoreInstigator) (Utilities|Array|MakeArray (Variables|Actor|GetInstigator)) 0)))
  (for _array_element _outactors
    (Default|CallOnAoeOverlapActor _array_element)
    (Development|PrintString (Utilities|GetDisplayName _array_element))))

(event EventBeginPlay
  (Utilities|FlowControl|Delay (Variables|Default|GetDelay))
  (CallFunction|SpawnAOESphere (Variables|Default|GetRadius))
  (Actor|DestroyActor))

(fn ConstructionScript)
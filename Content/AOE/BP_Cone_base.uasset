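; BP_Cone_base is a base area-of-effect actor that runs one cone overlap check from its Instigator after a delay, then destroys itself after a second delay.
; It tests the ConeCollide component's shape against Pawns at the Instigator's location and yaw-offset facing, broadcasting OnConeOverlapActor per hit.
; Length and Radius only size the optional debug cone, not the unit-scale overlap.
; The Instigator is ignored whatever IgnoreInstigator says.
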(event Custom|SpawnCone
  (params (Length :type Float%20%28double-precision%29) (Radius :type Float%20%28double-precision%29))
  (bind _instigator (Variables|Actor|GetInstigator))
  (bind _instigator_2 (Variables|Actor|GetInstigator))
  (bind _returnvalue (Transformation|GetActorForwardVector _instigator_2))
  (bind _array (Utilities|Array|MakeArray _instigator_2))
  (bind _returnvalue_2 (Math|Conversions|RotationFromXVector _returnvalue))
  (if (Variables|Default|GetDrawDebug)
    (Class|KismetSystemLibrary|DrawDebugConeinDegrees (Transformation|GetActorLocation _instigator) (Transformation|GetActorForwardVector _instigator) (* Length 2e+01) Radius Radius 12 "(R=1.000000,G=1.000000,B=1.000000,A=1.000000)" 2.0 1.0))
  (bind _outactors (Collision|ComponentOverlapActors (Variables|Default|Getcone_collide) (Math|Transform|MakeTransform (Transformation|GetActorLocation _instigator_2) (Math|Rotator|MakeRotator (.roll _returnvalue_2) (.pitch _returnvalue_2) (- (.yaw _returnvalue_2) -9e+01)) (Math|Vector|MakeVector 1.0 1.0 1.0)) (Utilities|Array|MakeArray "ObjectTypeQuery3") 0 (select (Variables|Default|GetIgnoreInstigator) _array _array)))
  (for _array_element _outactors
    (Default|CallOnConeOverlapActor _array_element)
    (Development|PrintString (Utilities|GetDisplayName _array_element))))

(event EventBeginPlay
  (bind _delay (Variables|Default|GetDelay))
  (Utilities|FlowControl|Delay _delay)
  (CallFunction|SpawnCone (Variables|Default|GetLength) (Variables|Default|GetRadius))
  (Utilities|FlowControl|Delay _delay)
  (Actor|DestroyActor))

(fn ConstructionScript)